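; Spawner actor that lays out a row of coin pickups at even spacing along a spline.
; The construction script adds placeholder static meshes at each spline distance to preview the layout.
; On BeginPlay it destroys those meshes and spawns BP_InteractivePickup actors at the same points.
; Pickups spawn with local-space spline transforms, then attach to the spawner with KeepRelative so those transforms become relative to it.
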(event `self.ReceiveBeginPlay`
  (bind (_location_at_distance_along_spline _rotation_at_distance_along_spline) (`self.Return Spline Location And Rotation`))
  (for _array_element (`self.Coin Mesh Array`)
    (`ActorComponent.K2_DestroyComponent` _array_element))
  (for _index (range (+ (`KismetMathLibrary.FTrunc` (/ (`SplineComponent.GetSplineLength` (`self.Spline`)) (`self.Space Between Each Coin`))) 1))
    (set `self.Spline Point` _index)
    (bind _returnvalue (`|SpawnActorFromClass` "/Game/Blueprints/Interactives/BP_InteractivePickup.BP_InteractivePickup_C" (`KismetMathLibrary.MakeTransform` _location_at_distance_along_spline _rotation_at_distance_along_spline) "Undefined" "OverrideRootScale" null null))
    (`self.K2_AttachToActor` _returnvalue self "None" "KeepRelative" "KeepRelative" "KeepRelative" true)))

(fn `Return Spline Location And Rotation`
  (returns (`Location At Distance Along Spline` :type "Vector Structure") (`Rotation At Distance Along Spline` :type "Rotator Structure"))
  (bind _spline (`self.Spline`))
  (bind _returnvalue (* (`self.Spline Point`) (`self.Space Between Each Coin`)))
  (return (`SplineComponent.GetLocationAtDistanceAlongSpline` _spline _returnvalue "Local") (`SplineComponent.GetRotationAtDistanceAlongSpline` _spline _returnvalue "Local")))

(fn `UserConstructionScript`
  (bind (_location_at_distance_along_spline _rotation_at_distance_along_spline) (`self.Return Spline Location And Rotation`))
  (`KismetArrayLibrary.Array_Clear` (`self.Coin Mesh Array`))
  (for _index (range (+ (`KismetMathLibrary.FTrunc` (/ (`SplineComponent.GetSplineLength` (`self.Spline`)) (`self.Space Between Each Coin`))) 1))
    (set `self.Spline Point` _index)
    (bind _returnvalue (`AddComponent|NODE_AddStaticMeshComponent-0` :`RelativeTransform` (`KismetMathLibrary.MakeTransform` _location_at_distance_along_spline _rotation_at_distance_along_spline)))
    (`KismetArrayLibrary.Array_Add` (`self.Coin Mesh Array`) _returnvalue)))