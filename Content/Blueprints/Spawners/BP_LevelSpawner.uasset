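; BP_LevelSpawner lays spline mesh sections along a Spline at construction time, with no runtime logic.
; The Construction Script divides spline length by SectionLength and adds a SplineMeshComponent for each step.
; ReturnSplinePositionAndTangent samples local positions and tangents at each section's ends using the SplinePoint index.
; Its StartTangent and EndPosition output names are swapped, and the SetStartAndEnd wiring compensates.
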(fn `Return Spline Position and Tangent`
  (returns (`Start Position` :type "Vector Structure") (`Start Tangent` :type "Vector Structure") (`End Position` :type "Vector Structure") (`End Tangent` :type "Vector Structure"))
  (bind _spline (`self.Spline`))
  (bind _spline_2 (`self.Spline`))
  (bind _returnvalue (* (`self.Spline Point`) (`self.Section Length`)))
  (bind _returnvalue_2 (* (+ (`self.Spline Point`) 1) (`self.Section Length`)))
  (return (`SplineComponent.GetLocationAtDistanceAlongSpline` _spline_2 _returnvalue "Local") (`SplineComponent.GetLocationAtDistanceAlongSpline` _spline _returnvalue_2 "Local") (`SplineComponent.GetTangentAtDistanceAlongSpline` _spline_2 _returnvalue "Local") (`SplineComponent.GetTangentAtDistanceAlongSpline` _spline _returnvalue_2 "Local")))

(fn `UserConstructionScript`
  (bind (_start_position _start_tangent _end_position _end_tangent) (`self.Return Spline Position and Tangent`))
  (for _index (range (+ (`KismetMathLibrary.FTrunc` (/ (`SplineComponent.GetSplineLength` (`self.Spline`)) (`self.Section Length`))) 1))
    (set `self.Spline Point` _index)
    (bind _returnvalue (`AddComponent|NODE_AddSplineMeshComponent-0`))
    (`SplineMeshComponent.SetStartAndEnd` _returnvalue _start_position _end_position _start_tangent _end_tangent true)))