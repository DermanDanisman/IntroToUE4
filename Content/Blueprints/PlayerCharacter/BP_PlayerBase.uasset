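; BP_PlayerBase is a base player Blueprint that moves by physics forces and looks around with the mouse.
; MoveForward and MoveRight pass the camera's forward or right vector and the axis value to GetMovementDirection, which scales them by MoveSpeed.
; The result drives AddForce on the static mesh as a mass-independent acceleration, and the camera vector keeps its vertical component.
; Turn and LookUp feed controller yaw and pitch.
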(event `InputAxis|MoveForward`
  (params (AxisValue :type "Float (single-precision)"))
  ;[1 1 1] Player Movement
  (`PrimitiveComponent.AddForce` (`self.StaticMesh`) (`self.Get Movement Direction` (`SceneComponent.GetForwardVector` (`self.Camera`)) (`self.GetInputAxisValue`)) "None" true))

(event `InputAxis|Turn`
  (params (AxisValue :type "Float (single-precision)"))
  ;[1 1 1] Player Mouse Control
  (`self.AddControllerYawInput` AxisValue))

(event `InputAxis|LookUp`
  (params (AxisValue :type "Float (single-precision)"))
  ;[1 1 1] Player Mouse Control
  (`self.AddControllerPitchInput` AxisValue))

(event `InputAxis|MoveRight`
  (params (AxisValue :type "Float (single-precision)"))
  ;[1 1 1] Player Movement
  (`PrimitiveComponent.AddForce` (`self.StaticMesh`) (`self.Get Movement Direction` (`SceneComponent.GetRightVector` (`self.Camera`)) (`self.GetInputAxisValue`)) "None" true))

(fn `Get Movement Direction`
  (params (`Input Direction` :type "Vector Structure") (`Move Input Axis` :type "Float (double-precision)"))
  (returns (ReturnValue :type "Vector Structure"))
  (return (* (* `Input Direction` `Move Input Axis`) (`self.MoveSpeed`))))

(fn `UserConstructionScript`)