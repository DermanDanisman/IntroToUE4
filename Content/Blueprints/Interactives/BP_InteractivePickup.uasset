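; BP_InteractivePickup is a collectible that flies to the player and reports its collection to the game mode.
; When a BP_PlayerBase enters the magnetic radius collider, a sped-up timeline lerps the pickup from its start position to the player's current location, tracking movement each update.
; The Interact override runs the parent logic, calls PickupCollected on BP_GameModeBase, then destroys the actor.
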(event `self.ReceiveBeginPlay`
  (`TimelineComponent.SetPlayRate` (`self.Move To Player Timeline`) 1.5))

(event `self.MagneticRadiusCollider.OnComponentBeginOverlap`
  (params (OverlappedComponent :type "PrimitiveComponent Object Reference") (OtherActor :type "Actor Object Reference") (OtherComp :type "PrimitiveComponent Object Reference") (OtherBodyIndex :type Integer) (bFromSweep :type Boolean) (SweepResult :type "HitResult Structure (by ref)"))
  (bind _asbp_player_base (cast `/Game/Blueprints/PlayerCharacter/BP_PlayerBase` OtherActor))
  (set `self.Player Reference` _asbp_player_base)
  (set `self.Start Location` (`self.K2_GetActorLocation`))
  (bind (_direction _move_to_track) (`Timeline|Move To Player Timeline`)
    (:`Update`
      (`self.K2_SetActorLocation` (`KismetMathLibrary.VLerp` (`self.Start Location`) (`self.K2_GetActorLocation` (`self.Player Reference`)) _move_to_track)))))

(fn `Interact`
  (params (OverlappedActor :type "Actor Object Reference"))
  (`parent.Interact` OverlappedActor)
  (bind _asbp_game_mode_base (cast `/Game/Blueprints/GameMode/BP_GameModeBase` (`GameplayStatics.GetGameMode`)))
  (`/Game/Blueprints/GameMode/BP_GameModeBase.PickupCollected` _asbp_game_mode_base)
  (`self.K2_DestroyActor`))

(fn `UserConstructionScript`
  (`parent.UserConstructionScript`))