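; BP_InteractiveBase is a base interactive actor that triggers when the player overlaps its StaticMesh.
; The overlap event casts to BP_PlayerBase, stores the player reference and calls Interact.
; Interact plays InteractSound at the actor's location and spawns either a Niagara or Cascade effect there, chosen by the PlayNiagara flag.
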(event `self.StaticMesh.OnComponentBeginOverlap`
  (params (OverlappedComponent :type "PrimitiveComponent Object Reference") (OtherActor :type "Actor Object Reference") (OtherComp :type "PrimitiveComponent Object Reference") (OtherBodyIndex :type Integer) (bFromSweep :type Boolean) (SweepResult :type "HitResult Structure (by ref)"))
  (bind _asbp_player_base (cast `/Game/Blueprints/PlayerCharacter/BP_PlayerBase` OtherActor))
  (bind _output_get (set `self.Interacting Player Reference` _asbp_player_base))
  (`self.Interact` _output_get))

(fn `Interact`
  (params (OverlappedActor :type "Actor Object Reference"))
  (`GameplayStatics.PlaySoundAtLocation` (`self.Interact Sound`) (`self.K2_GetActorLocation`) (struct) 1.0 1.0 0.0 null null null)
  (if (`self.bPlayNiagara`)
    (`NiagaraFunctionLibrary.SpawnSystemAtLocation` (`self.Niagara Effect`) (`self.K2_GetActorLocation`))
    (else
      (`GameplayStatics.SpawnEmitterAtLocation` (`self.Cascade Effect`) (`self.K2_GetActorLocation`)))))

(fn `UserConstructionScript`)