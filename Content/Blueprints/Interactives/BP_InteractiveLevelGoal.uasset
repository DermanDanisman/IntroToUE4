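; Interactive level goal that ends the level as a success when interacted with.
; Its Interact function casts the game mode to BP_GameModeBase and, only while the player is playing, calls LevelOver with true.
; It then spawns a Niagara effect and plays the interact sound at its own location.
; The construction script only runs the parent's.
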(fn `Interact`
  (params (OverlappedActor :type "Actor Object Reference"))
  (bind _asbp_game_mode_base (cast `/Game/Blueprints/GameMode/BP_GameModeBase` (`GameplayStatics.GetGameMode`)))
  (if (`/Game/Blueprints/GameMode/BP_GameModeBase.Is Player Playing` _asbp_game_mode_base)
    (`/Game/Blueprints/GameMode/BP_GameModeBase.LevelOver` _asbp_game_mode_base true)
    (`NiagaraFunctionLibrary.SpawnSystemAtLocation` (`self.Niagara Effect`) (`self.K2_GetActorLocation`))
    (`GameplayStatics.PlaySoundAtLocation` (`self.Interact Sound`) (`self.K2_GetActorLocation`) (struct) 1.0 1.0 0.0 null null null)))

(fn `UserConstructionScript`
  (`parent.UserConstructionScript`))