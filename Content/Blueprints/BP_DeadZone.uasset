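; BP_DeadZone is a trigger volume that fails the level when the player enters it.
; On box overlap by a BP_PlayerBase, it checks that BP_GameModeBase reports the player as playing, then calls LevelOver with false and plays the LevelFail sound at its location.
; The construction script applies the BoxExtent variable to the box, so each instance can be sized separately.
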(event `self.Box.OnComponentBeginOverlap`
  (params (OverlappedComponent :type "PrimitiveComponent Object Reference") (OtherActor :type "Actor Object Reference") (OtherComp :type "PrimitiveComponent Object Reference") (OtherBodyIndex :type Integer) (bFromSweep :type Boolean) (SweepResult :type "HitResult Structure (by ref)"))
  (cast `/Game/Blueprints/PlayerCharacter/BP_PlayerBase` OtherActor)
  (bind _asbp_game_mode_base (cast `/Game/Blueprints/GameMode/BP_GameModeBase` (`GameplayStatics.GetGameMode`)))
  (if (`/Game/Blueprints/GameMode/BP_GameModeBase.Is Player Playing` _asbp_game_mode_base)
    (`/Game/Blueprints/GameMode/BP_GameModeBase.LevelOver` _asbp_game_mode_base false)
    (`GameplayStatics.PlaySoundAtLocation` "/Game/Assets/Audio/LevelFail.LevelFail" (`self.K2_GetActorLocation`) (struct) 1.0 1.0 0.0 null null null)))

(fn `UserConstructionScript`
  (`BoxComponent.SetBoxExtent` (`self.Box`) (`self.Box Extent`) true))